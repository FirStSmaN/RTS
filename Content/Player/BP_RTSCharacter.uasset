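; Player character Blueprint for an RTS with Organism and Disease teams; its graph holds only number-key debug hooks.
; Key 1 traces from the camera toward the mouse position at Z=0, damages the hit RTSSelectAndMoveCharacter, then prints its health and controller.
; Key 2 prints both teams' title counts from the game mode.
; Keys 3 and 4 request each team's respawn unit from a found BP_BaseTitle's respawn component.
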(event `self.ReceiveBeginPlay`)

(event `Key|One`
  (params (Key :type "Key Structure"))
  (:`Pressed`
    (bind _returnvalue (`WidgetLayoutLibrary.GetMousePositionOnPlatform`))
    (`WidgetLayoutLibrary.GetMousePositionOnViewport`)
    (bind _outhit (`KismetSystemLibrary.LineTraceSingle` :`Start` (`SceneComponent.K2_GetComponentLocation` (`self.CameraComponent`)) :`End` (`KismetMathLibrary.Conv_Vector2DToVector` _returnvalue) :`TraceChannel` "TraceTypeQuery2" :`DrawDebugType` "ForDuration"))
    (bind (_bblockinghit _binitialoverlap _time _distance _location _impactpoint _normal _impactnormal _physmat _hitactor) (`GameplayStatics.BreakHitResult` _outhit))
    (bind _asrtsselect_and_move_character (cast `RTSSelectAndMoveCharacter` _hitactor))
    (`GameplayStatics.ApplyPointDamage` _asrtsselect_and_move_character 10.0 _location _outhit)
    (`KismetSystemLibrary.PrintText` (`KismetTextLibrary.Conv_DoubleToText` (`RTSAIHealthComponent.GetHealthPercent` (`RTSSelectAndMoveCharacter.HealthComponent` _asrtsselect_and_move_character)) "HalfToEven"))
    (`KismetSystemLibrary.PrintText` (`KismetTextLibrary.Conv_StringToText` (`KismetSystemLibrary.GetDisplayName` (`self.GetController` _asrtsselect_and_move_character))))))

(event `Key|Two`
  (params (Key :type "Key Structure"))
  (:`Pressed`
    (bind _asrtsgame_mode_base (cast `RTSGameModeBase` (`GameplayStatics.GetGameMode`))
      (:`then`
        (`KismetSystemLibrary.PrintString` (`KismetStringLibrary.Concat_StrStr` "Organism Titles Count:   " (`KismetStringLibrary.Conv_IntToString` (`KismetArrayLibrary.Array_Length` (`RTSTeamComponent.Titles` (`RTSGameModeBase.OrganismTeamComponent` _asrtsgame_mode_base))))))
        (`KismetSystemLibrary.PrintString` (`KismetStringLibrary.Concat_StrStr` "Disease Titles Count:   " (`KismetStringLibrary.Conv_IntToString` (`KismetArrayLibrary.Array_Length` (`RTSTeamComponent.Titles` (`RTSGameModeBase.DiseaseTeamComponent` _asrtsgame_mode_base)))))))
      (:`CastFailed`
        (`KismetSystemLibrary.PrintString` "Error")))))

(event `Key|Three`
  (params (Key :type "Key Structure"))
  (:`Pressed`
    (bind _returnvalue (`GameplayStatics.GetActorOfClass` "/Game/Titles/BP_BaseTitle.BP_BaseTitle_C"))
    (bind _returnvalue_2 (`BaseTitle.GetRespawnComponent` _returnvalue))
    (bind _asrtsgame_mode_base (cast `RTSGameModeBase` (`GameplayStatics.GetGameMode`)))
    (bind _returnvalue_3 (`RTSRespawnComponent.GetUnitToRespawn` _returnvalue_2 (`RTSGameModeBase.OrganismTeamComponent` _asrtsgame_mode_base)))
    (if (`KismetSystemLibrary.IsValid` _returnvalue_3)
      (`KismetSystemLibrary.PrintString` "Spawned"))))

(event `Key|Four`
  (params (Key :type "Key Structure"))
  (:`Pressed`
    (bind _returnvalue (`GameplayStatics.GetActorOfClass` "/Game/Titles/BP_BaseTitle.BP_BaseTitle_C"))
    (bind _returnvalue_2 (`BaseTitle.GetRespawnComponent` _returnvalue))
    (bind _asrtsgame_mode_base (cast `RTSGameModeBase` (`GameplayStatics.GetGameMode`)))
    (bind _returnvalue_3 (`RTSRespawnComponent.GetUnitToRespawn` _returnvalue_2 (`RTSGameModeBase.DiseaseTeamComponent` _asrtsgame_mode_base)))
    (if (`KismetSystemLibrary.IsValid` _returnvalue_3)
      (`KismetSystemLibrary.PrintString` "Spawned"))))

(fn `UserConstructionScript`)